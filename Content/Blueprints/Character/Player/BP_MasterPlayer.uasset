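; Master player character Blueprint handling movement, mouse look with sensitivity, crouch toggle, hold-to-run and jump.
; Running cancels on strafe or non-forward input, and jumping is blocked while strafing or moving backward.
; Tick derives an Idle/Walk/Run state from velocity and prints it for debugging.
; Movement axis events read that state through paired DoOnce gates to start camera shake on Walk and stop it on Idle.
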(event `InputAction|Crouch`
  (params (Key :type "Key Structure"))
  ;[1 1 1] Locomotion
  (:`Pressed`
    (if (`self.IsCrounch`)
      (`self.UnCrouch`)
      (set `self.IsCrounch` false)
      (else
        (`self.Crouch`)
        (set `self.IsCrounch` true)))))

(event `InputAction|Run`
  (params (Key :type "Key Structure"))
  ;[1 1 1] Locomotion
  (:`Pressed`
    (set `CharacterMovementComponent.MaxWalkSpeed` (`self.RunSpeed`) (`self.CharacterMovement`))
    (set `self.IsRunning` true))
  (:`Released`
    (set `CharacterMovementComponent.MaxWalkSpeed` (`self.WalkSpeed`) (`self.CharacterMovement`))
    (set `self.IsRunning` false)))

(event `InputAction|Jump`
  (params (Key :type "Key Structure"))
  ;[1 1 1] Locomotion
  (:`Pressed`
    (if (and (>= (`self.GetInputAxisValue`) 0.0) (== (`self.GetInputAxisValue`) 0.0))
      (`self.Jump`)))
  (:`Released`
    (`self.StopJumping`)))

(event `InputAxis|MoveForward`
  (params (AxisValue :type "Float (single-precision)"))
  ;[1 1 1] Locomotion
  (`self.AddMovementInput` (`SceneComponent.GetForwardVector` (`self.CapsuleComponent`)) AxisValue)
  (`|ExecutionSequence`
    (:`then_0`
      (switch `/Game/Blueprints/DATA/Enum/Enum_PlayerState` (`self.E_PlayerState`) :!label _label
        (:`NewEnumerator0`
          (`/Engine/EditorBlueprintResources/StandardMacros.DoOnce` false :!label _label_2
            (:`Completed`
              (`self.StopCameraShake`)
              (goto _label_3 :!via `Reset`))))
        (:`NewEnumerator1`
          (`/Engine/EditorBlueprintResources/StandardMacros.DoOnce` false :!label _label_3
            (:`Completed`
              (`self.StartCamShake`)
              (goto _label_2 :!via `Reset`))))))
    (:`then_1`
      (if (<= (`self.GetInputAxisValue`) 0.0)
        (`self.StopRunning`)))))

(event `InputAxis|MoveRight`
  (params (AxisValue :type "Float (single-precision)"))
  ;[1 1 1] Locomotion
  (`self.AddMovementInput` (`SceneComponent.GetRightVector` (`self.CapsuleComponent`)) AxisValue)
  (`|ExecutionSequence`
    (:`then_0`
      (goto _label))
    (:`then_1`
      (if (!= (`self.GetInputAxisValue`) 0.0)
        (`self.StopRunning`)))))

(event `InputAxis|LookUp`
  (params (AxisValue :type "Float (single-precision)"))
  ;[1 1 1] Locomotion
  (`self.AddControllerPitchInput` (* AxisValue (`self.MouseSensitivity`))))

(event `InputAxis|Turn`
  (params (AxisValue :type "Float (single-precision)"))
  ;[1 1 1] Locomotion
  (`self.AddControllerYawInput` (* AxisValue (`self.MouseSensitivity`))))

(event `self.ReceiveTick`
  (params (DeltaSeconds :type "Float (single-precision)"))
  (`|ExecutionSequence`
    (:`then_0`
      (`self.StateLocomotion`))
    (:`then_1`
      (`KismetSystemLibrary.PrintString` (`|GetEnumeratorNameAsString` (`self.E_PlayerState`))))))

(event `StartCamShake`
  (bind _returnvalue (`PlayerCameraManager.StartCameraShake` :`self` (`GameplayStatics.GetPlayerCameraManager` 0) :`ShakeClass` "/Game/Blueprints/DATA/Others/CameraShake.CameraShake_C")))

(event `StopCameraShake`
  (`PlayerCameraManager.StopCameraShake` (`GameplayStatics.GetPlayerCameraManager` 0) (stale `StartCamShake` _returnvalue) false))

(fn `StateLocomotion`
  (bind _returnvalue (`KismetMathLibrary.VSize` (`self.GetVelocity`)))
  (if (== _returnvalue 0.0)
    (set `self.E_PlayerState` "NewEnumerator0")
    (elif (> _returnvalue (+ (`self.WalkSpeed`) 5.0))
      (set `self.E_PlayerState` "NewEnumerator2")
      (elif (< _returnvalue (`self.RunSpeed`))
        (set `self.E_PlayerState` "NewEnumerator1")))))

(fn `StopRunning`
  (set `CharacterMovementComponent.MaxWalkSpeed` (`self.WalkSpeed`) (`self.CharacterMovement`))
  (set `self.IsRunning` false))

(fn `UserConstructionScript`)