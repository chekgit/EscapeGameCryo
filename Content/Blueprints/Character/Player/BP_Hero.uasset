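; BP_Hero is the player hero Blueprint, which sets up camera pitch limits when play begins.
; BeginPlay calls InitCamera, which applies the hero's min and max pitch variables to player 0's camera manager, then assigns CrouchSpeed from a same-named value.
; The construction script only calls its parent, and overlap and tick events are unused.
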(event `self.ReceiveBeginPlay`
  (`self.InitCamera`)
  (set `self.CrouchSpeed` (`self.CrouchSpeed`)))

(fn `InitCamera`
  (bind _returnvalue (`GameplayStatics.GetPlayerCameraManager` 0))
  (set `PlayerCameraManager.ViewPitchMin` (`self.PitchMinCam`) _returnvalue)
  (set `PlayerCameraManager.ViewPitchMax` (`self.PitchMaxCam`) _returnvalue))

(fn `UserConstructionScript`
  (`parent.UserConstructionScript`))