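; Base item Blueprint for objects the player can pick up to observe, with configurable name, mesh, mass and gravity.
; Interact disables physics and plays a timeline that lerps the item to a target point while spinning it over a given duration.
; De-interact reverses that timeline back to the saved transform.
; When the timeline finishes, it notifies the player character, re-enabling physics on return if gravity is enabled.
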(event `self.ReceiveBeginPlay`
  (`self.Switch Gravity` true))

(event `/Game/Blueprints/DATA/Interfaces/BPI_Interactable.Interact`
  (params (PointToReach :type "Vector Structure") (TimeToReach :type "Float (single-precision)") (TurnUpToReach :type "Float (single-precision)"))
  (bind _returnvalue (* 360 TurnUpToReach))
  (bind _returnvalue_2 (`GameplayStatics.GetPlayerCharacter` 0))
  (set `self.Interact/Deinteract` true)
  (`TimelineComponent.SetPlayRate` (`self.Timeline_MoveItemToObs`) (/ 1.0 TimeToReach))
  (`self.Switch Gravity` false)
  (bind _output_get (set `self.ActorTansformBeforeObs` (`self.GetTransform`)))
  (bind (_direction _alpha) (`Timeline|Timeline_MoveItemToObs` :!label _label)
    (:`Update`
      (`self.K2_SetActorLocationAndRotation` (`KismetMathLibrary.VLerp` (.location _output_get) PointToReach _alpha) (`KismetMathLibrary.RLerp` (.rotation _output_get) (`KismetMathLibrary.MakeRotator` (.roll (.rotation _output_get)) (+ (.pitch (.rotation _output_get)) _returnvalue) (+ (.yaw (.rotation _output_get)) _returnvalue)) _alpha)))
    (:`Finished`
      ;[1 1 1] Quand timeline terminée
      (if (`self.Interact/Deinteract`)
        (message `/Game/Blueprints/DATA/Interfaces/BPI_Interactable.TransitionObsFinished` _returnvalue_2)
        (else
          (message `/Game/Blueprints/DATA/Interfaces/BPI_Interactable.De-interact` _returnvalue_2)
          (`self.Switch Gravity` true))))))

(event `ReverseTimelineMoveObs`
  (goto _label :!via `Reverse`))

(event `/Game/Blueprints/DATA/Interfaces/BPI_Interactable.De-interact`
  (set `self.Interact/Deinteract` false)
  (`self.ReverseTimelineMoveObs`))

(fn `GetNameItem`
  (returns (NomItem :type Name))
  (return (`self.NomItem`)))

(fn `Switch Gravity`
  (params (Enable :type Boolean))
  (bind _staticmesh (`self.StaticMesh`))
  (bind _returnvalue (and (`self.EnableGravity`) Enable))
  (`PrimitiveComponent.SetSimulatePhysics` _staticmesh _returnvalue)
  (`PrimitiveComponent.SetEnableGravity` _staticmesh _returnvalue)
  (if Enable
    (`PrimitiveComponent.SetMassOverrideInKg` (`self.StaticMesh`) "None" (`self.Mass`) true)))

(fn `UserConstructionScript`
  (`StaticMeshComponent.SetStaticMesh` (`self.StaticMesh`) (`self.MeshAppearence`))
  (`TextRenderComponent.K2_SetText` (`self.TextForDebug`) (`|FormatText` "{NomItem} \nFace \n(Debug)" (`self.NomItem`))))