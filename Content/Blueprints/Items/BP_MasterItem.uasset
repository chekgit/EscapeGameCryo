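; Master item actor with configurable mesh, name, mass and gravity that the player can pick up for close observation.
; Interact disables physics and plays a timeline moving the item to a given point, oriented toward the camera with optional spins.
; De-interact reverses that timeline, then notifies the player character and restores physics.
; While observed, a looping per-frame timer rotates the item in fixed steps following mouse movement direction.
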(event `self.ReceiveBeginPlay`
  (`self.Switch Gravity` true))

(event `/Game/Blueprints/DATA/Interfaces/BPI_Interactable.Interact`
  (params (PointToReach :type "Vector Structure") (TimeToReach :type "Float (single-precision)") (TurnUpToReach :type Integer))
  (bind _returnvalue (`GameplayStatics.GetPlayerCharacter` 0))
  (bind _actortansformbeforeobs_location (`KismetMathLibrary.BreakTransform` (`self.ActorTansformBeforeObs`)))
  (bind (_actortansformbeforeobs_location_2 _actortansformbeforeobs_rotation) (`KismetMathLibrary.BreakTransform` (`self.ActorTansformBeforeObs`)))
  (bind (_actortransformafterobs_location _actortransformafterobs_rotation) (`KismetMathLibrary.BreakTransform` (`self.ActorTransformAfterObs`)))
  (bind _returnvalue_2 (`KismetMathLibrary.Conv_IntToDouble` (* TurnUpToReach 360)))
  ;[1 1 1] Mode Observation - LANCEMENT
  (set `self.Interact/Deinteract` true)
  (`TimelineComponent.SetPlayRate` (`self.Timeline_MoveItemToObs`) (/ 1.0 TimeToReach))
  (`self.Switch Gravity` false)
  (set `self.ActorTansformBeforeObs` (`self.GetTransform`))
  (bind (_direction _alpha) (`Timeline|Timeline_MoveItemToObs` :!label _label)
    (:`Update`
      (`self.K2_SetActorLocationAndRotation` (`KismetMathLibrary.VLerp` _actortansformbeforeobs_location PointToReach _alpha) (`KismetMathLibrary.RLerp` _actortansformbeforeobs_rotation (select `bool` (`self.Interact/Deinteract`) :`false` _actortransformafterobs_rotation :`true` (`KismetMathLibrary.MakeRotator` (.roll (`KismetMathLibrary.FindLookAtRotation` PointToReach (`PlayerCameraManager.GetCameraLocation` (`GameplayStatics.GetPlayerCameraManager` 0)))) (+ (.pitch (`KismetMathLibrary.FindLookAtRotation` PointToReach (`PlayerCameraManager.GetCameraLocation` (`GameplayStatics.GetPlayerCameraManager` 0)))) _returnvalue_2) (+ (.yaw (`KismetMathLibrary.FindLookAtRotation` PointToReach (`PlayerCameraManager.GetCameraLocation` (`GameplayStatics.GetPlayerCameraManager` 0)))) _returnvalue_2))) _alpha))
      ;[1 1 1] Orientation caméra sur demande en mode observation
      (`self.K2_AddActorLocalRotation` (select `bool` (`self.Interact/Deinteract`) :`true` (`KismetMathLibrary.RLerp` (struct) (`KismetMathLibrary.NegateRotator` (`SceneComponent.RelativeRotation` (`self.DirectionCamObservation`))) _alpha true))))
    (:`Finished`
      ;[1 1 1] Quand timeline terminée : Interaction ou Dé-intéraction ?
      (if (`self.Interact/Deinteract`)
        (message `/Game/Blueprints/DATA/Interfaces/BPI_Interactable.TransitionObsFinished` _returnvalue)
        (else
          (message `/Game/Blueprints/DATA/Interfaces/BPI_Interactable.De-interact` _returnvalue 0.0)
          (`self.Switch Gravity` true))))))

(event `ReverseTimelineMoveObs`
  (params (TimeToDeReachObs :type "Float (double-precision)"))
  (`TimelineComponent.SetPlayRate` (`self.Timeline_MoveItemToObs`) (/ 1.0 TimeToDeReachObs))
  (goto _label :!via `Reverse`))

(event `/Game/Blueprints/DATA/Interfaces/BPI_Interactable.De-interact`
  (params (TimeToDeReachObs :type "Float (single-precision)"))
  ;[1 1 1] Mode Observation - QUITTER
  (set `self.Interact/Deinteract` false)
  (set `self.ActorTransformAfterObs` (`self.GetTransform`))
  (`self.ReverseTimelineMoveObs` TimeToDeReachObs))

(event `/Game/Blueprints/DATA/Interfaces/BPI_Interactable.TurnItemObs`
  (params (`On/Off` :type Boolean))
  ;[1 1 1] Mode Observation - Faire tourner l'item
  (if `On/Off`
    (`KismetSystemLibrary.K2_SetTimer` self "TurnItemInOMode" (`GameplayStatics.GetWorldDeltaSeconds`) true)
    (else
      (`KismetSystemLibrary.K2_ClearTimer` self "TurnItemInOMode"))))

(fn `GetNameItem`
  (returns (NomItem :type Name))
  (return (`self.NomItem`)))

(fn `Switch Gravity`
  (params (Enable :type Boolean))
  (bind _staticmesh (`self.StaticMesh`))
  (bind _returnvalue (and (`self.EnableGravity`) Enable))
  (`PrimitiveComponent.SetSimulatePhysics` _staticmesh _returnvalue)
  (`PrimitiveComponent.SetEnableGravity` _staticmesh _returnvalue)
  (if Enable
    (`PrimitiveComponent.SetMassOverrideInKg` (`self.StaticMesh`) "None" (`self.Mass`) true)))

(fn `TurnItemInOMode`
  (locals (TurnXObs :type "Float (double-precision)") (TurnYObs :type "Float (double-precision)"))
  (bind _returnvalue (`WidgetLayoutLibrary.GetMousePositionOnPlatform`))
  (bind (_x _y) (`KismetMathLibrary.BreakVector2D` _returnvalue))
  (set `local.TurnXObs` _x)
  (set `local.TurnYObs` _y)
  (`|ExecutionSequence`
    (:`then_0`
      (`/Engine/EditorBlueprintResources/StandardMacros.DoOnce` (`self.LV_FirstTickOmode`)
        (:`Completed`
          (set `self.LV_FirstTickOmode` true)
          (set `self.LV_TurnXobsMemory` (`local.TurnXObs`))
          (set `self.LV_TurnYobsMemory` (`local.TurnYObs`)))))
    (:`then_1`
      (`/Engine/EditorBlueprintResources/StandardMacros.CompareFloat` (`local.TurnXObs`) (`self.LV_TurnXobsMemory`)
        (:`>`
          (`self.K2_AddActorLocalRotation` (struct :`Yaw` -1.0)))
        (:`<`
          (`self.K2_AddActorLocalRotation` (struct :`Yaw` 1.0))))
      (set `self.LV_TurnXobsMemory` (`local.TurnXObs`)))
    (:`then_2`
      (`/Engine/EditorBlueprintResources/StandardMacros.CompareFloat` (`local.TurnYObs`) (`self.LV_TurnYobsMemory`)
        (:`>`
          (`self.K2_AddActorLocalRotation` (struct :`Pitch` -1.0)))
        (:`<`
          (`self.K2_AddActorLocalRotation` (struct :`Pitch` 1.0))))
      (set `self.LV_TurnYobsMemory` (`local.TurnYObs`)))))

(fn `UserConstructionScript`
  (`StaticMeshComponent.SetStaticMesh` (`self.StaticMesh`) (`self.MeshAppearence`))
  (`TextRenderComponent.K2_SetText` (`self.TextForDebug`) (`|FormatText` "{NomItem} \nFace \n(Debug)" (`self.NomItem`))))