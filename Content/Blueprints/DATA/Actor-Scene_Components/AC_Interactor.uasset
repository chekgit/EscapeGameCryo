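; Actor component that lets its owner interact with objects in front of its camera when AC_Interact is called.
; It traces from the camera along its forward vector, using either a sphere or line trace on Visibility, ignoring the owner.
; A hit actor tagged "Interactable" that implements BPI_Interactable receives InteractionMessage.
; The owner needs both Camera and SpringArm components, otherwise an error prints, though the live trace ignores arm length.
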(event `AC_Interact`
  (bind _returnvalue (`self.GetOwner`))
  (bind _cameraactor (`self.CameraActor`))
  (bind _returnvalue_2 (`Actor.K2_GetComponentsByClass` _returnvalue "/Script/Engine.SpringArmComponent"))
  (bind (_bblockinghit _binitialoverlap _time _distance _location _impactpoint _normal _impactnormal _physmat _hitactor) (`GameplayStatics.BreakHitResult` (`self.Out Hit`)))
  (bind _returnvalue_3 (`SceneComponent.K2_GetComponentLocation` _cameraactor))
  (bind _returnvalue_4 (`Actor.K2_GetComponentsByClass` _returnvalue "/Script/Engine.CameraComponent"))
  (bind _array (`|MakeArray` (`self.GetOwner`)))
  (if (and (`KismetArrayLibrary.Array_IsValidIndex` _returnvalue_4) (`KismetArrayLibrary.Array_IsValidIndex` _returnvalue_2))
    (set `self.CameraActor` (`|GetArrayItem` _returnvalue_4))
    (set `self.SpringArmActor` (`|GetArrayItem` _returnvalue_2))
    (set `self.Start` _returnvalue_3)
    (set `self.End` (+ _returnvalue_3 (* (`SceneComponent.GetForwardVector` _cameraactor) (`self.Longueur_Trace`))))
    ;[1 1 1] TRACE
    (if (`self.IsSphereTrace`)
      (bind (_outhit _returnvalue_5) (`KismetSystemLibrary.SphereTraceSingle` (`self.Start`) (`self.End`) (`self.RadiusSphereTrace`) "TraceTypeQuery1" false _array (`self.Draw Debug Type`)))
      (if _returnvalue_5
        (set `self.Out Hit` _outhit)
        ;[1 1 1] RESULT
        (if (`Actor.ActorHasTag` _hitactor "Interactable") :!label _label
          (if (`KismetSystemLibrary.DoesImplementInterface` _hitactor "/Game/Blueprints/DATA/Interfaces/BPI_Interactable.BPI_Interactable_C")
            (message `/Game/Blueprints/DATA/Interfaces/BPI_Interactable.Interaction` _hitactor))))
      (else
        (bind (_outhit_2 _returnvalue_6) (`KismetSystemLibrary.LineTraceSingle` (`self.Start`) (`self.End`) "TraceTypeQuery1" false _array (`self.Draw Debug Type`)))
        (if _returnvalue_6
          (set `self.Out Hit` _outhit_2)
          (goto _label))))
    (else
      (`KismetSystemLibrary.PrintString` "L'acteur qui souhaite intéragir ne possède pas de Camera + SpringArm" true true (struct :`R` 1.0 :`A` 1.0) 5.0))))