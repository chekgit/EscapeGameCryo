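; Actor component that detects which interactable the owning actor's camera faces and notifies it when focus is gained or lost.
; A looping timer, started on BeginPlay and toggled by a function, sphere-traces forward from the camera (zero radius if disabled); the owner needs Camera and SpringArm components.
; Hits with a tagged AC_Interactable implementing BPI_Interactable trigger interaction/de-interaction messages on component and actor, with DoOnce gates preventing repeats.
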(event `self.ReceiveBeginPlay`
  ;[1 1 1] Lancement de l'interact
  (`self.AC_Des-activate_interaction` true))

(fn `AC_Des-activate_interaction`
  (params (Activation :type Boolean))
  (bind _timer_interaction (`self.Timer_Interaction`))
  (if Activation
    (if (not (`KismetSystemLibrary.K2_IsValidTimerHandle` (`self.Timer_Interaction`)))
      (bind _returnvalue (`KismetSystemLibrary.K2_SetTimer` self "AC_Interaction" (`self.TimeToUpdateInteraction`) true))
      (set `self.Timer_Interaction` _returnvalue))
    (elif (`KismetSystemLibrary.K2_IsValidTimerHandle` _timer_interaction)
      (`KismetSystemLibrary.K2_ClearAndInvalidateTimerHandle` _timer_interaction)
      ;[1 1 1] Reset des variables
      (set `self.Last_Hit_Actor_Interactable` null)
      (set `self.Out Hit` (struct)))))

(fn `AC_Interaction`
  (bind _returnvalue (`self.GetOwner`))
  (bind _last_hit_actor_interactable (`self.Last_Hit_Actor_Interactable`))
  (bind _cameraactor (`self.CameraActor`))
  (bind _returnvalue_2 (`Actor.K2_GetComponentsByClass` _returnvalue "/Script/Engine.SpringArmComponent"))
  (bind _returnvalue_3 (`SceneComponent.K2_GetComponentLocation` _cameraactor))
  (bind _returnvalue_4 (`Actor.K2_GetComponentsByClass` _returnvalue "/Script/Engine.CameraComponent"))
  (if (and (`KismetArrayLibrary.Array_IsValidIndex` _returnvalue_4) (`KismetArrayLibrary.Array_IsValidIndex` _returnvalue_2))
    (set `self.CameraActor` (`|GetArrayItem` _returnvalue_4))
    (set `self.SpringArmActor` (`|GetArrayItem` _returnvalue_2))
    (set `self.Start` _returnvalue_3)
    (set `self.End` (+ _returnvalue_3 (* (`SceneComponent.GetForwardVector` _cameraactor) (`self.Longueur_Trace`))))
    ;[1 1 1] TRACE
    (if (not (`self.IsSphereTrace`))
      (set `self.RadiusSphereTrace` 0.0))
    (bind (_outhit _returnvalue_5) (`KismetSystemLibrary.SphereTraceSingle` (`self.Start`) (`self.End`) (`self.RadiusSphereTrace`) "TraceTypeQuery1" false (`|MakeArray` (`self.GetOwner`)) (`self.Draw Debug Type`)))
    (if _returnvalue_5
      (bind (_bblockinghit _binitialoverlap _time _distance _location _impactpoint _normal _impactnormal _physmat _hitactor) (`GameplayStatics.BreakHitResult` _outhit))
      (bind _returnvalue_6 (`Actor.GetComponentByClass` _hitactor "/Game/Blueprints/DATA/ActorComponents/AC_Interactable.AC_Interactable_C"))
      ;[1 1 1] RESULT
      (`/Engine/EditorBlueprintResources/StandardMacros.IsValid` _returnvalue_6
        (:`Is Valid`
          (if (and (`self.ComponentHasTag` _returnvalue_6 "Interactable") (`KismetSystemLibrary.DoesImplementInterface` _returnvalue_6 "/Game/Blueprints/DATA/Interfaces/BPI_Interactable.BPI_Interactable_C"))
            (`|ExecutionSequence`
              (:`then_0`
                ;;[0.1275 1 0.1756] Gestion intéraction
                (`/Engine/EditorBlueprintResources/StandardMacros.DoOnce` (`self.DoOnceInteractClosed`)
                  (:`Completed`
                    ;;;[1 1 1] Gestion des DoOnce dans la fonction "locale"
                    (set `self.DoOnceDeinteractClosed` false)
                    (set `self.DoOnceInteractClosed` true)
                    (bind _output_get (set `self.Out Hit` _outhit))
                    (bind _output_get_2 (set `self.Last_Hit_Actor_Interactable` (`.HitActor` (`GameplayStatics.BreakHitResult` _output_get))))
                    ;;;[1 1 1] Interaction AC pour réaction commune
                    (message `/Game/Blueprints/DATA/Interfaces/BPI_Interactable.Interaction` (`Actor.GetComponentByClass` _output_get_2 "/Game/Blueprints/DATA/ActorComponents/AC_Interactable.AC_Interactable_C"))
                    (if (`KismetSystemLibrary.DoesImplementInterface` _last_hit_actor_interactable "/Game/Blueprints/DATA/Interfaces/BPI_Interactable.BPI_Interactable_C")
                      ;;;[1 1 1] Interaction Actor pour réaction spécifique
                      (message `/Game/Blueprints/DATA/Interfaces/BPI_Interactable.Interaction` _last_hit_actor_interactable)))))
              (:`then_1`
                ;;[1 0.4928 0.2708] Verif : Passage d'un item interactable à un autre
                (if (and (`self.DoOnceInteractClosed`) (!= _hitactor (`self.Last_Hit_Actor_Interactable`)))
                  ;;[1 0.2917 0.2917] Gestion dé-intéraction
                  (`/Engine/EditorBlueprintResources/StandardMacros.DoOnce` (`self.DoOnceDeinteractClosed`) :!label _label
                    (:`Completed`
                      ;;;[1 1 1] Gestion des DoOnce dans la fonction "locale"
                      (set `self.DoOnceDeinteractClosed` true)
                      (set `self.DoOnceInteractClosed` false)
                      (set `self.Out Hit` (struct))
                      ;;;[1 1 1] De-intéraction AC pour réaction commune
                      (message `/Game/Blueprints/DATA/Interfaces/BPI_Interactable.De-interaction` (`Actor.GetComponentByClass` (`self.Last_Hit_Actor_Interactable`) "/Game/Blueprints/DATA/ActorComponents/AC_Interactable.AC_Interactable_C"))
                      ;;;[1 1 1] De-intéraction Actor pour réaction spécifique
                      (message `/Game/Blueprints/DATA/Interfaces/BPI_Interactable.De-interaction` (`self.Last_Hit_Actor_Interactable`)))))))
            (else
              (goto _label))))
        (:`Is Not Valid`
          (goto _label)))
      (else
        (goto _label)))
    (else
      (`KismetSystemLibrary.PrintString` "L'acteur qui souhaite intéragir ne possède pas de Camera + SpringArm" true true (struct :`R` 1.0 :`A` 1.0) 5.0))))